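; Zombie enemy that endlessly chases the player and attacks in melee until killed.
; AI MoveTo leads into an attack montage, whose notify runs a sphere overlap at an arrow component to damage the first-person character.
; Completed or interrupted attacks loop back to the chase, via a hit reaction when interrupted, so being shot doesn't stall it.
; Point damage lowers health, triggering hit reactions or death, which stops movement and destroys the capsule.
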(event Custom|RunToPlayer
  ;[1 1 1 1 45] zombie chase player
  (if (not (Variables|Default|GetisDead?))
    (AI|AIMoveTo self "0, 0, 0" (Game|GetPlayerController 0) 4e+01 false
      (:OnSuccess
        (CallFunction|AttackPlayer))
      (:OnFail
        (CallFunction|RuntoPlayer)))))

(event Custom|AttackPlayer
  ;[1 1 1 1 45] zombie attack and anim logic
  (Animation|Montage|PlayMontage (Variables|Character|GetMesh) "/Game/_Main/zombie/Anims/Zombie_Attack_Montage.Zombie_Attack_Montage" 1.5
    (:OnCompleted
      (CallFunction|RuntoPlayer))
    (:OnInterrupted
      ;;[0.4115 0 0 1 30] to fix the issue that zombie stops chasing player when we interrupt the zombies' attack animation by shooting at them
      (Animation|Montage|PlayMontage (Variables|Character|GetMesh) "/Game/_Main/zombie/Anims/Zombie_Reaction_Hit_Montage.Zombie_Reaction_Hit_Montage"
        (:OnCompleted
          (CallFunction|RuntoPlayer))
        (:OnInterrupted
          (CallFunction|RuntoPlayer))))
    (:OnNotifyBegin
      (bind (_outactors _returnvalue) (Collision|SphereOverlapActors (Transformation|GetWorldLocation (Variables|Default|GetArrow1)) 8e+01 (Utilities|Array|MakeArray "ObjectTypeQuery3") "/Game/_Main/Blueprints/BP_FirstPersonCharacter.BP_FirstPersonCharacter_C" (Utilities|Array|MakeArray self)))
      (if _returnvalue
        (for _array_element _outactors
          (Game|Damage|ApplyDamage _array_element 2e+01 (Pawn|GetController) self "/Script/Engine.DamageType"))))))

(event Custom|ZombieDeath
  ;[1 1 1 1 45] zombie death logic
  (Variables|Default|SetisDead? true)
  (Components|Movement|StopMovementImmediately (Variables|Character|GetCharacterMovement))
  (Animation|Montage|PlayMontage (Variables|Character|GetMesh) "/Game/_Main/zombie/Anims/Zombie_Death_Montage.Zombie_Death_Montage" 1.5
    (:then
      (Components|DestroyComponent (Variables|Collision|GetCapsuleComponent)))))

(event EventBeginPlay
  ;[1 1 1 1 50] Event begin
  (CallFunction|RuntoPlayer))

(event Game|Damage|EventPointDamage
  (params (Damage :type Float%20%28single-precision%29) (DamageType :type Damage%20Type%20Object%20Reference) (HitLocation :type Vector :default "0, 0, 0") (HitNormal :type Vector :default "0, 0, 0") (HitComponent :type Primitive%20Component%20Object%20Reference) (BoneName :type Name :default "None") (ShotFromDirection :type Vector :default "0, 0, 0") (InstigatedBy :type Controller%20Object%20Reference) (DamageCauser :type Actor%20Object%20Reference) (HitInfo :type Hit%20Result%20Structure%20%28by%20ref%29))
  ;[1 1 1 1 45] Apply damage to Zombie logic
  (if (not (Variables|Default|GetisDead?))
    (if (<= (Variables|Default|Gethealth) 0.0)
      (CallFunction|ZombieDeath)
      (else
        (bind _output_get (Variables|Default|Sethealth (- (Variables|Default|Gethealth) Damage)))
        (Development|PrintString (Utilities|String|ToString(Float) _output_get))
        (if (<= _output_get 0.0)
          (CallFunction|ZombieDeath)
          (else
            (Animation|Montage|PlayMontage (Variables|Character|GetMesh) "/Game/_Main/zombie/Anims/Zombie_Reaction_Hit_Montage.Zombie_Reaction_Hit_Montage")))))))

(fn ConstructionScript)