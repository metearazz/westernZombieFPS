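; GameModeZombie is a game mode Blueprint that spawns a wave of zombies when play begins.
; Wave1 calls itself on a two-second delay, spawning BP_zombie at one of two randomly chosen locations and counting each spawn.
; Tick sets WaveLimit once the count reaches CurrentWave times WaveSpawnLimit, which stops the loop.
; The graph contains no logic to reset the limit or advance the wave.
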(event Custom|StartGame
  ;[1 1 1 1 50] Start Game
  (CallFunction|Wave1))

(event Custom|Wave1
  ;[1 1 1 1 50] Spawn Zombies
  (if (not (Variables|Default|GetwaveLimit))
    (Game|SpawnActorfromClass "/Game/_Main/zombie/BP_zombie.BP_zombie_C" (.OutItem (Utilities|Array|Random (Utilities|Array|MakeArray (Variables|Default|GetspawnLocation1) (Variables|Default|GetspawnLocation2)))) "Undefined" "MultiplyWithRoot" 0 0)
    (bind _result (Math|Integer|IncrementInt (Variables|Default|GetzombiesSpawnedSinceStart))
      (:%20%20
        (Variables|Default|SetzombiesSpawnedSinceStart _result)
        (Utilities|FlowControl|Delay 2.0)
        (CallFunction|Wave1)))))

(event EventBeginPlay
  ;[1 1 1 1 50] Start Game
  (CallFunction|StartGame))

(event EventTick
  (params (DeltaSeconds :type Float%20%28single-precision%29))
  ;[1 1 1 1 50] Spawn Zombies
  ;;[1 1 1 1 50] Check wave spawn limit reached
  (if (>= (Variables|Default|GetzombiesSpawnedSinceStart) (* (Variables|Default|GetcurrentWave) (Variables|Default|GetwaveSpawnLimit)))
    (Variables|Default|SetwaveLimit true)))

(fn ConstructionScript)